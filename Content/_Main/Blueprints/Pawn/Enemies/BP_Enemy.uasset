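; BP_Enemy is an enemy pawn Blueprint that repeatedly fires rockets, alternating between two gun sockets on its mesh.
; Tick runs a Delay of FireRate as a repeating timer, then a FlipFlop calls Fire with SocketNameR or SocketNameL.
; Fire spawns a BP_EnemyRocket at that socket's world transform and also sets SocketNameR to "Gun_R".
; BeginPlay, Tick and the construction script call their parent implementations.
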(event `self.ReceiveBeginPlay`
  (`parent.ReceiveBeginPlay`))

(event `self.ReceiveTick`
  (params (DeltaSeconds :type "Float (single-precision)"))
  (`parent.ReceiveTick` DeltaSeconds)
  (`KismetSystemLibrary.Delay` (`self.FireRate`))
  (if true
    (`/Engine/EditorBlueprintResources/StandardMacros.FlipFlop`
      (:`A`
        (`self.Fire` (`self.SocketName_R`)))
      (:`B`
        (`self.Fire` (`self.SocketName_L`))))))

(fn `Fire`
  (params (SocketName :type Name))
  (if true
    (set `self.SocketName_R` "Gun_R")
    (`|SpawnActorFromClass` "/Game/_Main/Blueprints/Pawn/Projectiles/BP_EnemyRocket.BP_EnemyRocket_C" (`SceneComponent.GetSocketTransform` (`self.EnemyMesh`) SocketName "RTS_World") "Undefined" "MultiplyWithRoot" null null)
    (else
      (set `self.SocketName_R` "Gun_L"))))

(fn `UserConstructionScript`
  (`parent.UserConstructionScript`))