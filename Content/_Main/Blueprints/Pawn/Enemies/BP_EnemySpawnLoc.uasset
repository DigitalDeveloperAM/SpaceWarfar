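; Enemy spawner that runs up to three sequential waves of enemies.
; A looping timer starts the next wave once the GM_SpaceWarfar game mode reports no enemies alive.
; StartWave passes the wave size to the game mode, then WaveSpawn spawns that many random classes from the wave's array at once.
; Spawn positions share the game mode's minimum X and Y, with Z randomized between its bounds.
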(event `self.ReceiveBeginPlay`
  ;[0.01764 0.01764 0.01764] Spawn Waves
  (bind _asgm_space_warfar (cast `/Game/_Main/Blueprints/GameModes/GM_SpaceWarfar` (`GameplayStatics.GetGameMode`)))
  (set `self.GameMode` _asgm_space_warfar)
  (bind _returnvalue (`KismetSystemLibrary.K2_SetTimer` null "CheckWaves" 0.5 true))
  (set `self.WaveTimer` _returnvalue))

(event `CheckWaves`
  (bind _output (`|GetArrayItem` (`self.EnemyWaveNum`) (`self.IndexWave`)))
  (bind _output_2 (`|GetArrayItem` (`self.EnemyWaveNum`) (`self.IndexWave`)))
  (bind _output_3 (`|GetArrayItem` (`self.EnemyWaveNum`) (`self.IndexWave`)))
  (if (and (== (`/Game/_Main/Blueprints/GameModes/GM_SpaceWarfar.AliveEnemies` (`self.GameMode`)) 0) (`self.WaveStart`))
    (switch `int` (`self.IndexWave`)
      (:`0`
        (`self.StartWave` _output_2)
        (`self.WaveSpawn` _output_2 (`self.EnmeyWaveOne`)))
      (:`1`
        (`self.StartWave` _output_3)
        (`self.WaveSpawn` _output_3 (`self.EnmeyWaveTwo`)))
      (:`2`
        (`self.StartWave` _output)
        (`self.WaveSpawn` _output (`self.EnmeyWaveThree`))))
    (set `self.IndexWave` (+ (`self.IndexWave`) 1))))

(fn `StartWave`
  (params (TotalWave :type Integer))
  (bind _gamemode (`self.GameMode`))
  (set `self.WaveStart` false)
  (set `self.ActiveWave` 0)
  (set `/Game/_Main/Blueprints/GameModes/GM_SpaceWarfar.MaxDistance` TotalWave _gamemode)
  (set `/Game/_Main/Blueprints/GameModes/GM_SpaceWarfar.CurrentWave` TotalWave _gamemode))

(fn `UserConstructionScript`)

(fn `WaveSpawn`
  (params (TotalWave :type Integer) (EnemeisWave :type "Array of /Game/_Main/Blueprints/Pawn/Enemies/BP_EnemyBase Class Reference"))
  (bind _gamemode (`self.GameMode`))
  (bind (_maxenemiesspawnloc_x _maxenemiesspawnloc_y _maxenemiesspawnloc_z) (`KismetMathLibrary.BreakVector` (`/Game/_Main/Blueprints/GameModes/GM_SpaceWarfar.MaxEnemiesSpawnLoc` _gamemode)))
  (bind (_minenemiesspawnloc_x _minenemiesspawnloc_y _minenemiesspawnloc_z) (`KismetMathLibrary.BreakVector` (`/Game/_Main/Blueprints/GameModes/GM_SpaceWarfar.MinEnemiesSpawnLoc` _gamemode)))
  (for _ (range (+ (+ TotalWave 1) 1))
    (if (> TotalWave (`self.ActiveWave`))
      (if (not (`self.WaveStart`))
        (`|SpawnActorFromClass` (`|GetArrayItem` EnemeisWave (`KismetMathLibrary.RandomInteger` (`KismetArrayLibrary.Array_Length` EnemeisWave))) (`KismetMathLibrary.MakeTransform` (`KismetMathLibrary.MakeVector` _minenemiesspawnloc_x _minenemiesspawnloc_y (`KismetMathLibrary.RandomFloatInRange` _minenemiesspawnloc_z _maxenemiesspawnloc_z))) "Undefined" "MultiplyWithRoot" null null)
        (set `self.ActiveWave` (+ (`self.ActiveWave`) 1)))
      (else
        (set `self.WaveStart` true)))))