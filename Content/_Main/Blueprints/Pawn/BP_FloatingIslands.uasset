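; BP_FloatingIslands is an island actor that scrolls from right to left across the screen in the space warfare game mode.
; Each Tick moves the root a fixed step along negative Y, without scaling by delta time.
; Once past the left screen bound, it stops moving, waits a random short delay, asks GM_SpaceWarfar to spawn islands, then destroys itself.
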(event `self.ReceiveTick`
  (params (DeltaSeconds :type "Float (single-precision)"))
  (bind (_returnvalue_x _returnvalue_y) (`KismetMathLibrary.BreakVector` (`SceneComponent.K2_GetComponentLocation` (`self.DefaultSceneRoot`))))
  ;[0.01764 0.01764 0.01764] Island movement from the right to left.
  (if (< _returnvalue_y (`self.OutLeftScreen`))
    (`KismetSystemLibrary.Delay` (`KismetMathLibrary.RandomFloatInRange` 1.0 3.0))
    (bind _asgm_space_warfar (cast `/Game/_Main/Blueprints/GameModes/GM_SpaceWarfar` (`GameplayStatics.GetGameMode`)))
    (`/Game/_Main/Blueprints/GameModes/GM_SpaceWarfar.SpawnIslands` _asgm_space_warfar)
    (`self.K2_DestroyActor`)
    (else
      ;;[0.01764 0.01764 0.01764] Speed of the island movement in Y.
      (`SceneComponent.K2_AddWorldOffset` (`self.DefaultSceneRoot`) (0.0 -200.0 0.0) false false))))

(fn `UserConstructionScript`)