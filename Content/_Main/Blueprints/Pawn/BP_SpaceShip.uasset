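; Player spaceship pawn that moves, fires guns and rockets, and ends the game in a win or loss.
; BeginPlay plays a spinning fly-in, creates the HUD, loads win/loss totals and starts looping health-regen and distance timers.
; Tick smooths input into swept movement with banking, while Enhanced Input events spawn projectiles at ship sockets, with rocket cooldown.
; Lethal damage shows game over; reaching the distance goal shows victory, saves totals and pauses.
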(event `EnhancedInput|/Game/_Main/Blueprints/Inputs/IA_RocketFire`
  (params (ActionValue :type Boolean) (ElapsedSeconds :type "Float (double-precision)") (TriggeredSeconds :type "Float (double-precision)") (InputAction :type "InputAction Object Reference" :default "/Game/_Main/Blueprints/Inputs/IA_RocketFire.IA_RocketFire"))
  ;[0.01764 0.01764 0.01764] Fire Rocket Press Right Mouse Key
  (:`Started`
    (if (<= (`self.RocketCoolDown`) 0.0)
      (`KismetSystemLibrary.Delay` 2.0)
      (set `self.RocketCoolDown` (`self.RocketMaxCoolDown`))
      (else
        (`self.RocketFire`)
        (set `self.RocketCoolDown` 0.0)))))

(event `EnhancedInput|/Game/_Main/Blueprints/Inputs/IA_Fire`
  (params (ActionValue :type Boolean) (ElapsedSeconds :type "Float (double-precision)") (TriggeredSeconds :type "Float (double-precision)") (InputAction :type "InputAction Object Reference" :default "/Game/_Main/Blueprints/Inputs/IA_Fire.IA_Fire"))
  ;[0.01764 0.01764 0.01764] Fire Gun Press Left Mouse Key
  (:`Started`
    (`/Engine/EditorBlueprintResources/StandardMacros.FlipFlop`
      (:`A`
        (`self.Fire`))
      (:`B`
        (`self.Fire`)))))

(event `FireProjectileBeam`
  ;[0.01764 0.01764 0.01764] Spawn Projectile inffinity.
)

(event `self.ReceiveBeginPlay`
  (bind _returnvalue (`GameplayStatics.GetPlayerController` 0))
  (bind _startloc (`self.StartLoc`))
  (`|ExecutionSequence`
    (:`then_0`
      ;[0.01764 0.01764 0.01764] Enhanced Inputs
      (bind _asplayer_controller (cast `PlayerController` (`GameplayStatics.GetPlayerController` 0)))
      (`EnhancedInputSubsystemInterface.AddMappingContext` (pcsubsystem `EnhancedInputLocalPlayerSubsystem` _asplayer_controller) "/Game/_Main/Blueprints/Inputs/IMC_SpaceWarfar.IMC_SpaceWarfar" 0 (struct)))
    (:`then_1`
      ;[0.01764 0.01764 0.01764] Spawn Animation.
      (set `self.Health` (`self.MaxHealth`))
      (set `self.RocketCoolDown` (`self.RocketMaxCoolDown`))
      (set `self.Pitch` (.roll (`SceneComponent.RelativeRotation` (`self.SpaceShip`))))
      (set `self.StartRotation` (`SceneComponent.K2_GetComponentRotation` (`self.SpaceShip`)))
      (set `self.StartLoc` (`self.K2_GetActorLocation`))
      (bind (_direction _spawn) (`Timeline|SpawnAnimation`)
        (:`Update`
          (`self.K2_SetActorLocation` (`KismetMathLibrary.VLerp` _startloc (+ _startloc (0.0 2000.0 0.0)) _spawn))
          (`SceneComponent.K2_SetRelativeRotation` (`self.SpaceShip`) (`KismetMathLibrary.RLerp` (`self.StartRotation`) (`KismetMathLibrary.MakeRotator` 0.0 (+ 720.0 (`self.Pitch`))) _spawn) false false))
        (:`Finished`
          (set `self.isMoving` true))))
    (:`then_2`
      ;[0.01764 0.01764 0.01764] Game HUD
      (bind _returnvalue_2 (`|CreateWidget` "/Game/_Main/Blueprints/Widgets/W_HUD.W_HUD_C"))
      (bind _output_get (set `self.WidgetRef` _returnvalue_2))
      (`UserWidget.AddToViewport` _output_get 0)
      ;[0.01764 0.01764 0.01764] Regenerted health every 2.0S by 10
      (`KismetSystemLibrary.Delay` 2.0)
      (`KismetSystemLibrary.K2_SetTimer` null "HealthRegenerted" 2.0 true))
    (:`then_3`
      ;[0.01764 0.01764 0.01764] Distance counter.
      (`KismetSystemLibrary.K2_SetTimer` null "IncrementCounter" 0.25 true))
    (:`then_4`
      ;[0.01764 0.01764 0.01764] Get controller back when start the game again.
      (set `PlayerController.bShowMouseCursor` false _returnvalue)
      (`WidgetBlueprintLibrary.SetInputMode_GameOnly` _returnvalue))
    (:`then_5`
      ;[0.01764 0.01764 0.01764] Save Game For Wins And Loss
      (`GameplayStatics.DoesSaveGameExist` "NumberOfWins")
      (if true
        (bind _returnvalue_3 (`GameplayStatics.LoadGameFromSlot` "NumberOfWins"))
        (bind _assg_save_game (cast `/Game/_Main/Blueprints/Saves/SG_SaveGame` _returnvalue_3))
        (set `self.TotalNumberWins` (`/Game/_Main/Blueprints/Saves/SG_SaveGame.WinsNum` _assg_save_game))
        (set `self.TotalNumLoss` (`/Game/_Main/Blueprints/Saves/SG_SaveGame.LossNum` _assg_save_game))))))

(event `self.ReceiveTick`
  (params (DeltaSeconds :type "Float (single-precision)"))
  ;[0.01764 0.01764 0.01764] Movement for the Pawn
  (set `self.DeltaSeconds` DeltaSeconds)
  (if (`self.isMoving`)
    (`|ExecutionSequence`
      (:`then_0`
        (bind _return (`self.Directions` (`self.UpSpeed`) (`|GetInputActionValue`)))
        (set `self.UpSpeed` _return))
      (:`then_1`
        (bind _return_2 (`self.Directions` (`self.RightSpeed`) (`|GetInputActionValue`)))
        (set `self.RightSpeed` _return_2))
      (:`then_2`
        (`self.K2_SetActorLocation` (+ (`self.K2_GetActorLocation`) (`KismetMathLibrary.MakeVector` 0.0 0.0 (`self.UpSpeed`))) true)
        (`self.K2_SetActorLocation` (+ (`self.K2_GetActorLocation`) (`KismetMathLibrary.MakeVector` 0.0 (`self.RightSpeed`))) true)
        (if (> (`self.Health`) 0.0)
          (`SceneComponent.K2_SetRelativeRotation` (`self.SpaceShip`) (`KismetMathLibrary.RInterpTo` (`self.K2_GetActorRotation`) (`KismetMathLibrary.MakeRotator` 0.0 (`self.RightSpeed`)) (`self.DeltaSeconds`) 20.0) false false))))))

(event `self.ReceiveAnyDamage`
  (params (Damage :type "Float (single-precision)") (DamageType :type "DamageType Object Reference") (InstigatedBy :type "Controller Object Reference") (DamageCauser :type "Actor Object Reference"))
  (bind _returnvalue (`GameplayStatics.GetPlayerController` 0))
  ;[0.01764 0.01764 0.01764] Player Death
  (bind _output_get (set `self.Health` (`KismetMathLibrary.FClamp` (- (`self.Health`) Damage) 0.0 (`self.MaxHealth`))))
  (if (<= _output_get 0.0)
    (bind _asgm_space_warfar (cast `/Game/_Main/Blueprints/GameModes/GM_SpaceWarfar` (`GameplayStatics.GetGameMode`)))
    (set `/Game/_Main/Blueprints/GameModes/GM_SpaceWarfar.isDead?` true _asgm_space_warfar)
    (`self.K2_DestroyActor`)
    ;[1 0 0] Update Lossing on Screen Works Not Working on UI Bug Fix Later
    (bind _output_get_2 (set `self.TotalNumLoss` (+ (`self.TotalNumLoss`) 1)))
    (`KismetSystemLibrary.PrintString` (`KismetStringLibrary.Concat_StrStr` "Loss: " (`KismetStringLibrary.Conv_IntToString` _output_get_2)))
    ;[0.01764 0.01764 0.01764] Game Over.
    (bind _returnvalue_2 (`|CreateWidget` "/Game/_Main/Blueprints/Widgets/W_GameOver.W_GameOver_C"))
    (`UserWidget.AddToViewport` _returnvalue_2 0)
    (set `PlayerController.bShowMouseCursor` true _returnvalue)
    (`WidgetBlueprintLibrary.SetInputMode_UIOnlyEx` _returnvalue _returnvalue_2)))

(fn `AddScore`
  (set `self.PlayerScore` (+ (`self.PlayerScore`) 1)))

(fn `Directions`
  (params (Speed :type "Float (double-precision)") (Direction :type "Float (double-precision)"))
  (returns (Return :type "Float (double-precision)"))
  ;[0.01764 0.01764 0.01764] Muliplacation 4k to DeltaTime and interp smooth it.
  (bind _output_get (set `self.CurrentSpeed` (`KismetMathLibrary.FInterpTo` Speed (* (* Direction (`self.MovementSpeed`)) (`self.DeltaSeconds`)) (`self.DeltaSeconds`) 4.0)))
  (return _output_get))

(fn `Fire`
  (if true
    (set `self.SocketName` "Gun_R")
    (else
      (set `self.SocketName` "Gun_L")))
  (`|SpawnActorFromClass` "/Game/_Main/Blueprints/Pawn/Projectiles/BP_GunProjectile.BP_GunProjectile_C" (`SceneComponent.GetSocketTransform` (`self.SpaceShip`) (`self.SocketName`) "RTS_World") "Undefined" "MultiplyWithRoot" null null))

(fn `HealthRegenerted`
  (if (<= (`self.Health`) 100.0)
    (set `self.Health` (+ (`self.Health`) (`self.RegenHealthAmount`)))))

(fn `IncrementCounter`
  (bind _returnvalue (`GameplayStatics.GetPlayerController` 0))
  (bind _output_get (set `self.DistanceCounter` (+ (`self.DistanceCounter`) 1)))
  (bind _returnvalue_2 (>= _output_get 10000))
  (if _returnvalue_2
    (`KismetSystemLibrary.K2_ClearTimer` null "IncrementCounter")
    (if _returnvalue_2
      ;[0.01764 0.01764 0.01764] Winning Widget End Game
      (bind _returnvalue_3 (`|CreateWidget` "/Game/_Main/Blueprints/Widgets/W_Win.W_Win_C"))
      (`UserWidget.AddToViewport` _returnvalue_3 0)
      (set `PlayerController.bShowMouseCursor` true _returnvalue)
      (`WidgetBlueprintLibrary.SetInputMode_UIOnlyEx` _returnvalue _returnvalue_3)
      (set `self.TotalNumberWins` (+ (`self.TotalNumberWins`) 1))
      (`self.SaveWinsNumber`)
      (`GameplayStatics.SetGamePaused` true))))

(fn `RocketFire`
  (if true
    (set `self.SocketName` "Gun_R")
    (else
      (set `self.SocketName` "Gun_L")))
  (`|SpawnActorFromClass` "/Game/_Main/Blueprints/Pawn/Projectiles/BP_Rocket.BP_Rocket_C" (`SceneComponent.GetSocketTransform` (`self.SpaceShip`) (`self.SocketName`) "RTS_World") "Undefined" "MultiplyWithRoot" null null))

(fn `SaveWinsNumber`
  (bind _totalnumloss (`self.TotalNumLoss`))
  (bind _totalnumberwins (`self.TotalNumberWins`))
  (bind _returnvalue (`GameplayStatics.DoesSaveGameExist` "NumberOfWins"))
  (if _returnvalue
    (bind _returnvalue_2 (`GameplayStatics.LoadGameFromSlot` "NumberOfWins"))
    (bind _assg_save_game (cast `/Game/_Main/Blueprints/Saves/SG_SaveGame` _returnvalue_2))
    (set `/Game/_Main/Blueprints/Saves/SG_SaveGame.WinsNum` _totalnumberwins _assg_save_game)
    (set `/Game/_Main/Blueprints/Saves/SG_SaveGame.LossNum` _totalnumloss _assg_save_game)
    (`GameplayStatics.SaveGameToSlot` _assg_save_game "NumberOfWins")
    (else
      (bind _returnvalue_3 (`GameplayStatics.CreateSaveGameObject` "/Game/_Main/Blueprints/Saves/SG_SaveGame.SG_SaveGame_C"))
      (set `/Game/_Main/Blueprints/Saves/SG_SaveGame.WinsNum` _totalnumberwins _returnvalue_3)
      (set `/Game/_Main/Blueprints/Saves/SG_SaveGame.LossNum` _totalnumloss _returnvalue_3)
      (`GameplayStatics.SaveGameToSlot` _returnvalue_3 "NumberOfWins"))))

(fn `SpawnProjectileBeam`
  (params (SocketName :type Name))
  (`|SpawnActorFromClass` "/Game/_Main/Blueprints/Pawn/Projectiles/BP_PorjectileBase.BP_PorjectileBase_C" (`SceneComponent.GetSocketTransform` (`self.SpaceShip`) SocketName "RTS_World") "Undefined" "MultiplyWithRoot" null null))

(fn `UserConstructionScript`)