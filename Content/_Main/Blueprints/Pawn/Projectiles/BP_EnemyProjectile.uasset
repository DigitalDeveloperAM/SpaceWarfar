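; BP_EnemyProjectile is an enemy-fired projectile that damages the player's spaceship on contact.
; Each tick it moves along its local offset by Speed scaled by delta time, without sweeping.
; When its mesh begins an overlap, it applies Damage only to a BP_SpaceShip, then destroys itself whatever it hit.
; The construction script sets the actor's scale from the Scale variable.
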(event `self.ReceiveTick`
  (params (DeltaSeconds :type "Float (single-precision)"))
  (`self.K2_AddActorLocalOffset` (* DeltaSeconds (`self.Speed`))))

(event `self.ProjectileMesh.OnComponentBeginOverlap`
  (params (OverlappedComponent :type "PrimitiveComponent Object Reference") (OtherActor :type "Actor Object Reference") (OtherComp :type "PrimitiveComponent Object Reference") (OtherBodyIndex :type Integer) (bFromSweep :type Boolean) (SweepResult :type "HitResult Structure (by ref)"))
  (bind _asbp_space_ship (cast `/Game/_Main/Blueprints/Pawn/BP_SpaceShip` OtherActor)
    (:`then`
      (`GameplayStatics.ApplyDamage` _asbp_space_ship (`self.Damage`)))
    (:`CastFailed`
      _))
  (`self.K2_DestroyActor`))

(fn `UserConstructionScript`
  (`self.SetActorScale3D` (`self.Scale`)))