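; Homing rocket projectile that seeks an enemy and damages it on contact.
; The Homing component locks onto the first BP_EnemyBase it overlaps while no valid target is held.
; Each tick, projectile velocity is lerped with a fixed overshooting alpha toward the target's direction scaled by AccelerationSpeed.
; Any mesh overlap destroys the rocket, applying BaseDamage first if the other actor is an enemy.
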(event `self.ReceiveTick`
  (params (DeltaSeconds :type "Float (single-precision)"))
  ;[0.01764 0.01764 0.01764] Calculate the distance between rocket and Enamy and boost the speed rocket & normalize first
  (`/Engine/EditorBlueprintResources/StandardMacros.IsValid` (`self.Enemy`)
    (:`Is Valid`
      (set `MovementComponent.Velocity` (`KismetMathLibrary.VLerp` (`MovementComponent.Velocity` (`self.ProjectileMovement`)) (* (`KismetMathLibrary.Normal` (- (`self.K2_GetActorLocation` (`self.Enemy`)) (`self.K2_GetActorLocation`))) (`self.AccelerationSpeed`)) 2.0) (`self.ProjectileMovement`)))))

(event `self.Homing.OnComponentBeginOverlap`
  (params (OverlappedComponent :type "PrimitiveComponent Object Reference") (OtherActor :type "Actor Object Reference") (OtherComp :type "PrimitiveComponent Object Reference") (OtherBodyIndex :type Integer) (bFromSweep :type Boolean) (SweepResult :type "HitResult Structure (by ref)"))
  ;[0.01764 0.01764 0.01764] Rocket Follows up the Enemy when get close.
  (bind _asbp_enemy_base (cast `/Game/_Main/Blueprints/Pawn/Enemies/BP_EnemyBase` OtherActor))
  (`/Engine/EditorBlueprintResources/StandardMacros.IsValid` (`self.Enemy`)
    (:`Is Not Valid`
      (set `self.Enemy` _asbp_enemy_base))))

(event `self.ProjectileMesh.OnComponentBeginOverlap`
  (params (OverlappedComponent :type "PrimitiveComponent Object Reference") (OtherActor :type "Actor Object Reference") (OtherComp :type "PrimitiveComponent Object Reference") (OtherBodyIndex :type Integer) (bFromSweep :type Boolean) (SweepResult :type "HitResult Structure (by ref)"))
  ;[0.01764 0.01764 0.01764] Enemy Death by rocket
  (bind _asbp_enemy_base (cast `/Game/_Main/Blueprints/Pawn/Enemies/BP_EnemyBase` OtherActor)
    (:`then`
      (`GameplayStatics.ApplyDamage` _asbp_enemy_base (`self.Base Damage`)))
    (:`CastFailed`
      _))
  (`self.K2_DestroyActor`))

(fn `UserConstructionScript`
  (`parent.UserConstructionScript`))