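; Enemy rocket projectile that damages the player spaceship on impact.
; Tick blends velocity toward a normalized direction to its Enemy target scaled by AccelerationSpeed, though the Lerp alpha is zero, so homing has no effect as written.
; Mesh overlap with BP_SpaceShip applies damage and triggers a camera shake through GM_SpaceWarfar before destroying the rocket.
; Overlap with any other actor simply destroys it.
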(event `self.ReceiveTick`
  (params (DeltaSeconds :type "Float (single-precision)"))
  ;[0.01764 0.01764 0.01764] Calculate the distance between rocket and Enamy and boost the speed rocket & normalize first
  (`/Engine/EditorBlueprintResources/StandardMacros.IsValid` (`self.Enemy`)
    (:`Is Valid`
      (set `MovementComponent.Velocity` (`KismetMathLibrary.VLerp` (`MovementComponent.Velocity` (`self.ProjectileMovement`)) (* (`KismetMathLibrary.Normal` (- (`self.K2_GetActorLocation` (`self.Enemy`)) (`self.K2_GetActorLocation`))) (`self.AccelerationSpeed`))) (`self.ProjectileMovement`)))))

(event `self.ProjectileMesh.OnComponentBeginOverlap`
  (params (OverlappedComponent :type "PrimitiveComponent Object Reference") (OtherActor :type "Actor Object Reference") (OtherComp :type "PrimitiveComponent Object Reference") (OtherBodyIndex :type Integer) (bFromSweep :type Boolean) (SweepResult :type "HitResult Structure (by ref)"))
  (bind _asbp_space_ship (cast `/Game/_Main/Blueprints/Pawn/BP_SpaceShip` OtherActor)
    (:`then`
      (`GameplayStatics.ApplyDamage` _asbp_space_ship (`self.Base Damage`))
      (bind _asgm_space_warfar (cast `/Game/_Main/Blueprints/GameModes/GM_SpaceWarfar` (`GameplayStatics.GetGameMode`)))
      (`/Game/_Main/Blueprints/GameModes/GM_SpaceWarfar.CameraShake` _asgm_space_warfar "/Game/_Main/Blueprints/Pawn/Effects/BP_CameraShake.BP_CameraShake_C"))
    (:`CastFailed`
      _))
  (`self.K2_DestroyActor`))

(fn `UserConstructionScript`
  (`parent.UserConstructionScript`))